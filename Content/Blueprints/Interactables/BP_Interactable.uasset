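; BP_Interactable is an interactable object that detects when the player is interacting with it.
; On BeginPlay, after a short delay, it caches references to the player pawn and game instance.
; InteractArea overlap events set a Touching flag for the player, and while that is true, Tick mirrors the player's Interacting state into InteractedWith.
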(event OnComponentEndOverlap(Interactarea)
  (params (OverlappedComponent :type Primitive%20Component%20Object%20Reference) (OtherActor :type Actor%20Object%20Reference) (OtherComp :type Primitive%20Component%20Object%20Reference) (OtherBodyIndex :type Integer))
  ;[0.05956 0.15 0.005032 0.5] Is the player touching the object?
  (if (== OtherActor (Variables|Default|GetplayerRefrence))
    (Variables|Default|SetTouching false)))

(event OnComponentBeginOverlap(Interactarea)
  (params (OverlappedComponent :type Primitive%20Component%20Object%20Reference) (OtherActor :type Actor%20Object%20Reference) (OtherComp :type Primitive%20Component%20Object%20Reference) (OtherBodyIndex :type Integer) (bFromSweep :type Boolean) (SweepResult :type Hit%20Result%20Structure%20%28by%20ref%29))
  ;[0.05956 0.15 0.005032 0.5] Is the player touching the object?
  (if (== OtherActor (Variables|Default|GetplayerRefrence))
    (Variables|Default|SetTouching true)))

(event EventBeginPlay
  ;[0.15 0.02558 0.04054 0.5] Create refrence to the player
  (Utilities|FlowControl|Delay 0.5)
  (bind _asbp_player (Utilities|Casting|CastToBP_Player (Game|Player|GetPlayerPawn 0)))
  (Variables|Default|SetplayerRefrence _asbp_player)
  ;[0.15 0.1079 0 0.5] Refrence to game instance
  (bind _asbp_game_instance (Utilities|Casting|CastToBP_GameInstance (Game|GetGameInstance)))
  (Variables|Default|SetGameInstance _asbp_game_instance))

(event EventTick
  (params (DeltaSeconds :type Float%20%28single-precision%29))
  ;[0.0323 0.15 0.1395 0.5] Has the object been interacted with
  (if (Variables|Default|GetTouching)
    (if (Variables|/Game/Blueprints/BP_Player.BP_Player_C|GetInteracting (Variables|Default|GetplayerRefrence))
      (Variables|Default|SetinteractedWith true)
      (else
        (Variables|Default|SetinteractedWith false)))))

(fn ConstructionScript)