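; BP_FishBase is the base Blueprint for an interactable fish that can be cut open with a knife.
; On BeginPlay it caches the player character and the level's BPI_DB_Knife actor, then tracks whether that knife overlaps it.
; Each tick it checks for knife contact while the player is interacting, marking the fish open once and printing debug messages for the cut or an already-open fish.
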(event Custom|Cut
  ;[0.1188 0 0.15 0.5] Cuts open the fish
  (if (Variables|Default|GetKnifeTouching)
    (if (Variables|/Game/Blueprints/BP_Player.BP_Player_C|GetInteracting (Variables|Default|GetPlayerReference))
      (if (Variables|Default|GetisOpen)
        (Development|PrintString "Already Open")
        (else
          (Development|PrintString "OW!")
          (Variables|Default|SetisOpen true))))))

(event EventBeginPlay
  ;[0.15 0.0165 0.09108 0.5] Gets refrence to player character
  (bind _asbp_player (Utilities|Casting|CastToBP_Player (Game|GetPlayerCharacter 0)))
  (Variables|Default|SetPlayerReference _asbp_player)
  ;[0.01003 0.05496 0.15 0.5] Knife reference
  (bind _returnvalue (Actor|GetActorOfClass "/Game/Blueprints/Interactables/Dragables/BPI_DB_Knife.BPI_DB_Knife_C"))
  (Variables|Default|SetKnifeReference _returnvalue))

(event EventTick
  (params (DeltaSeconds :type Float%20%28single-precision%29))
  ;[0.6948 0.0717 0 0.5] Checks for cut every tick
  (CallFunction|Cut))

(event Collision|EventActorBeginOverlap
  (params (OtherActor :type Actor%20Object%20Reference))
  ;[0.0182 0.15 0.1377 0.5] checks if the knife is touching the fish
  (if (== OtherActor (Variables|Default|GetKnifeReference))
    (Variables|Default|SetKnifeTouching true)))

(event Collision|EventActorEndOverlap
  (params (OtherActor :type Actor%20Object%20Reference))
  ;[0.0182 0.15 0.1377 0.5] checks if the knife is touching the fish
  (if (== OtherActor (Variables|Default|GetKnifeReference))
    (Variables|Default|SetKnifeTouching false)))

(fn ConstructionScript)