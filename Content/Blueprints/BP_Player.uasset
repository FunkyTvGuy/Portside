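; BP_Player is the player character, handling movement, jumping, interaction and mouse pick-up actions in the gutting level.
; BeginPlay adds the IMC_Player Enhanced Input mapping context, caches BP_GameInstance and notifies it that a level has loaded.
; Input events drive control-yaw-relative movement, call pick-up or put-down dispatchers, and briefly pulse an Interacting flag.
; A temporary dev key fades to black and opens the Testing level.
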(event Input|EnhancedActionEvents|EnhancedInputActionIA_Interact
  (params (ActionValue :type Boolean) (ElapsedSeconds :type Float%20%28double-precision%29) (TriggeredSeconds :type Float%20%28double-precision%29) (InputAction :type Input%20Action%20Object%20Reference :default "/Game/Inputs/IA_Interact.IA_Interact"))
  ;[0.02398 0.1136 0.15 0.5] Interact Button
  (Variables|Default|SetInteracting true)
  (Utilities|FlowControl|Delay 0.1)
  (Variables|Default|SetInteracting false))

(event Input|EnhancedActionEvents|EnhancedInputActionIA_MoveWorld
  (params (ActionValue :type Vector%202D%20Structure) (ElapsedSeconds :type Float%20%28double-precision%29) (TriggeredSeconds :type Float%20%28double-precision%29) (InputAction :type Input%20Action%20Object%20Reference :default "/Game/Inputs/IA_MoveWorld.IA_MoveWorld"))
  (bind _returnvalue (Pawn|GetControlRotation :!class /Script/Engine.Pawn))
  ;[0.15 0.02778 0.00228 0.5] WASD Movement
  (Pawn|Input|AddMovementInput (Math|Vector|GetRightVector (Math|Rotator|MakeRotator (.roll _returnvalue) 0.0 (.yaw _returnvalue))) (.x ActionValue) false)
  (Pawn|Input|AddMovementInput (Math|Vector|GetForwardVector (Math|Rotator|MakeRotator 0.0 0.0 (.yaw (Pawn|GetControlRotation :!class /Script/Engine.Pawn)))) (.y ActionValue) false))

(event Input|EnhancedActionEvents|EnhancedInputActionIA_TempDevButtons
  (params (ActionValue :type Boolean) (ElapsedSeconds :type Float%20%28double-precision%29) (TriggeredSeconds :type Float%20%28double-precision%29) (InputAction :type Input%20Action%20Object%20Reference :default "/Game/Inputs/IA_TempDevButtons.IA_TempDevButtons"))
  ;[0.15 0.15 0.15 0.5] Return to main level with 'R'
  (Default|FadetoBlack (Variables|Default|GetGameInstance))
  (Utilities|FlowControl|Delay 0.5)
  (Game|OpenLevel(byObjectReference) "/Game/Levels/testing.testing"))

(event Input|EnhancedActionEvents|EnhancedInputActionIA_AlanJump
  (params (ActionValue :type Boolean) (ElapsedSeconds :type Float%20%28double-precision%29) (TriggeredSeconds :type Float%20%28double-precision%29) (InputAction :type Input%20Action%20Object%20Reference :default "/Game/Inputs/IA_AlanJump.IA_AlanJump"))
  ;[0.05903 0.15 0.01915 0.5] Makes the player jump (dedicated to Alan <3)
  (:Triggered
    (Character|Jump))
  (:Completed
    (Character|StopJumping)))

(event Input|EnhancedActionEvents|EnhancedInputActionIA_MouseCursor
  (params (ActionValue :type Boolean) (ElapsedSeconds :type Float%20%28double-precision%29) (TriggeredSeconds :type Float%20%28double-precision%29) (InputAction :type Input%20Action%20Object%20Reference :default "/Game/Inputs/IA_MouseCursor.IA_MouseCursor"))
  ;[0.2756 1 0 0.5] Calls pickup/putdown dispatcher whenever player left clicks while in gutting level based on context from picked object
  (if (Variables|Default|GetInGuttingLevel)
    (if (Variables|Default|GetPickinIt)
      (Default|CallPickingUp)
      (else
        (Default|CallPuttingDown)))))

(event EventTick
  (params (DeltaSeconds :type Float%20%28single-precision%29))
  ;[0.1119 0.15 0.115 0.5] Is the player attemping to interact? DISABLED
)

(event EventBeginPlay
  ;[0.1463 0.15 0.02767 0.5] Sets up mapping context at start up
  (bind _asbp_player_controller (Utilities|Casting|CastToBP_PlayerController (Game|GetPlayerController 0)))
  (Utilities|IsValid (PlayerController|LocalPlayerSubsystems|GetEnhancedInputLocalPlayerSubsystem _asbp_player_controller)
    (:Is%20Valid
      (Input|AddMappingContext (PlayerController|LocalPlayerSubsystems|GetEnhancedInputLocalPlayerSubsystem _asbp_player_controller) "/Game/Inputs/IMC_Player.IMC_Player" 0 "(bIgnoreAllPressedKeysUntilRelease=True,bForceImmediately=False,bNotifyUserSettings=False)")
      ;[0.15 0.003341 0.09854 0.5] Tells the game instance to keep track of the current level
      (bind _asbp_game_instance (Utilities|Casting|CastToBP_GameInstance (Game|GetGameInstance)))
      (bind _output_get (Variables|Default|SetGameInstance _asbp_game_instance))
      (Default|LevelLoaded _output_get))))

(fn ConstructionScript)